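; BP_PowerUpOrb is a pickup orb that grants a damage boost, invincibility or healing, selected by EffectType.
; When BP_Player overlaps its collision, it forwards the effect to BP_WaveManager, destroys itself and refreshes the HUD.
; BeginPlay creates a dynamic material instance, which the ApplyVisualByType event recolors alongside setting a matching text label.
; ApplyVisualByType is not called within this Blueprint.
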(event OnComponentBeginOverlap(Collision)
  (params (OverlappedComponent :type Primitive%20Component%20Object%20Reference) (OtherActor :type Actor%20Object%20Reference) (OtherComp :type Primitive%20Component%20Object%20Reference) (OtherBodyIndex :type Integer) (bFromSweep :type Boolean) (SweepResult :type Hit%20Result%20Structure%20%28by%20ref%29))
  (bind _buffduration (Variables|Default|GetBuffDuration))
  (Utilities|Casting|CastToBP_Player OtherActor)
  (bind _returnvalue (Actor|GetActorOfClass "/Game/Game/Managers/BP_WaveManager.BP_WaveManager_C"))
  (Utilities|IsValid _returnvalue
    (:Is%20Valid
      (switch Utilities|FlowControl|Switch|SwitchonE_PowerUpType (Variables|Default|GetEffectType)
        (:NewEnumerator0
          (Default|ApplyDamagePowerUp _returnvalue (Variables|Default|GetDamageMultiplier) _buffduration))
        (:NewEnumerator1
          (Default|ApplyInvinciblePowerUp _returnvalue _buffduration))
        (:NewEnumerator2
          (Default|ApplyHealPowerUp _returnvalue (Variables|Default|GetHealAmount))))
      (Actor|DestroyActor)
      (Default|RefreshHUD _returnvalue))))

(event Custom|ApplyVisualByType
  (switch Utilities|FlowControl|Switch|SwitchonE_PowerUpType (Variables|Default|GetEffectType)
    (:NewEnumerator0
      (Rendering|Components|TextRender|SetText (Variables|Default|GetEffectText) (Utilities|Text|ToText(String) "DMG"))
      (Rendering|Material|SetVectorParameterValue (Variables|Default|GetOrbMaterial) "OrbColor" (Utilities|Struct|MakeLinearColor 1.0 0.1 0.05 1.0) :!class /Script/Engine.MaterialInstanceDynamic))
    (:NewEnumerator1
      (Rendering|Components|TextRender|SetText (Variables|Default|GetEffectText) (Utilities|Text|ToText(String) "INV"))
      (Rendering|Material|SetVectorParameterValue (Variables|Default|GetOrbMaterial) "OrbColor" (Utilities|Struct|MakeLinearColor 0.1 0.5 1.0 1.0) :!class /Script/Engine.MaterialInstanceDynamic))
    (:NewEnumerator2
      (Rendering|Components|TextRender|SetText (Variables|Default|GetEffectText) (Utilities|Text|ToText(String) "HEAL"))
      (Rendering|Material|SetVectorParameterValue (Variables|Default|GetOrbMaterial) "OrbColor" (Utilities|Struct|MakeLinearColor 0.0 1.0 0.2 1.0) :!class /Script/Engine.MaterialInstanceDynamic))))

(event Collision|EventActorBeginOverlap
  (params (OtherActor :type Actor%20Object%20Reference)))

(event EventTick
  (params (DeltaSeconds :type Float%20%28single-precision%29)))

(event EventBeginPlay
  (bind _returnvalue (Rendering|Material|CreateDynamicMaterialInstance (Variables|Default|GetOrbMesh) 0 "/Game/Game/Material/M_PowerUpOrb.M_PowerUpOrb" "None" :!class /Script/Engine.PrimitiveComponent))
  (Variables|Default|SetOrbMaterial _returnvalue))

(fn ConstructionScript)